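; SizeUpItemBP is a pickup that gives the player a size-up item when touched.
; On component overlap, it uses a stored Player reference, which it can fill by casting player 0's controlled pawn to PlayerBP.
; If the overlapping actor is that player, it calls GetSizeUpItem on the player and destroys itself.
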(event `self.SizeUpItem.OnComponentBeginOverlap`
  (params (OverlappedComponent :type "PrimitiveComponent Object Reference") (OtherActor :type "Actor Object Reference") (OtherComp :type "PrimitiveComponent Object Reference") (OtherBodyIndex :type Integer) (bFromSweep :type Boolean) (SweepResult :type "HitResult Structure (by ref)"))
  (bind _player (`self.Player`))
  ;[1 1 1] プレイヤーのサイズアップアイテム取得処理
  (if (not (!= null (`self.Player`)))
    (bind _asplayer_bp (cast `/Game/Player/BPFile/PlayerBP` (`Controller.K2_GetPawn` (`GameplayStatics.GetPlayerController` 0))))
    (set `self.Player` _asplayer_bp))
  (if (== OtherActor _player)
    (`/Game/Player/BPFile/PlayerBP.GetSizeUpItem` _player)
    (`self.K2_DestroyActor`)))

(fn `UserConstructionScript`)