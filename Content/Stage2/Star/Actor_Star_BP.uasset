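; Stage 2 star pickup actor that shatters when the player touches it and records the pickup in the game instance.
; BeginPlay binds to a fracture dispatcher on EventSendBP, which the player's overlap with the destructible mesh calls manually.
; That overlap also applies heavy upward damage to EventSendBP's destructible mesh to break it.
; The bound handler runs once, spawning star particles, adding audio and calling StarGet on SuperGameInstance.
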(event `self.ReceiveBeginPlay`
  (add `self.BindEventtoOnComponentFracture` (`self.eventSendBP`) (delegate `CustomEvent_0`)) ; 破壊イベントを取得
)

(event `CustomEvent_0`
  (`/Engine/EditorBlueprintResources/StandardMacros.DoOnce` false ; 1度だけ実行する
    (:`Completed`
      ;[1 1 1] はじけスター
      (`GameplayStatics.SpawnEmitterAtLocation` "/Game/Stage2/Effect/StarParticle.StarParticle" (`SceneComponent.K2_GetComponentLocation` (`self.Star_Breaker_DM`))) ; ParticleSistem
      (`AddComponent|NODE_AddAudioComponent-0`)
      (bind _assuper_game_instance (cast `/Game/UI/SuperGameInstance` (`GameplayStatics.GetGameInstance`)))
      (`/Game/UI/SuperGameInstance.StarGet` _assuper_game_instance))))

(event `self.Star_Breaker_DM.OnComponentBeginOverlap`
  (params (OverlappedComponent :type "PrimitiveComponent Object Reference") (OtherActor :type "Actor Object Reference") (OtherComp :type "PrimitiveComponent Object Reference") (OtherBodyIndex :type Integer) (bFromSweep :type Boolean) (SweepResult :type "HitResult Structure (by ref)"))
  (if (not (!= (`self.PlayerBP`) null))
    (bind _asplayer_bp (cast `/Game/Player/BPFile/PlayerBP` (`Controller.K2_GetPawn` (`GameplayStatics.GetPlayerController` 0))))
    (set `self.PlayerBP` _asplayer_bp))
  (if (== OtherActor (`self.PlayerBP`))
    (`self.BindEventtoOnComponentFracture` (`self.eventSendBP`)) ; Bindされたコマンドをすべて実行
    (`DestructibleComponent.ApplyDamage` (`/Game/Stage2/Star/Actor_Star_BP.Star_Breaker_DM` (`self.eventSendBP`)) 15000.0 (`self.K2_GetActorLocation` (`self.eventSendBP`)) (`KismetMathLibrary.MakeVector` 0.0 0.0 1.0) 15000.0) ; オーバーラップ中のダメージイベントを発生させる
  ))

(event `self.Star.OnComponentHit`
  (params (HitComponent :type "PrimitiveComponent Object Reference") (OtherActor :type "Actor Object Reference") (OtherComp :type "PrimitiveComponent Object Reference") (NormalImpulse :type "Vector Structure") (Hit :type "HitResult Structure (by ref)")))

(fn `UserConstructionScript`)