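; Player pawn for a rolling-ball character with HP, knockback damage and timed speed-up and size-up power-ups.
; Movement input builds camera-relative torque, which Tick applies only while a downward trace hits and speed is below the cap.
; Power-up and invincibility timers count down in that same branch, so they pause otherwise.
; Size-up blocks damage, and high velocity sets a speed-line flag in a material parameter collection.
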(event `self.ReceiveBeginPlay`
  (bind _returnvalue (`GameplayStatics.GetPlayerCameraManager` 0))
  ;[1 1 1] Initialization
  (set `PlayerCameraManager.ViewPitchMin` -40.0 _returnvalue)
  (set `PlayerCameraManager.ViewPitchMax` 0.0 _returnvalue)
  (`self.SetDefaultSpeed`)
  (`self.SetDefaultSize`)
  (set `self.PlayerHP` 5))

(event `InputAxis|MoveForward`
  (params (AxisValue :type "Float (single-precision)"))
  (bind _rolltorque (`self.RollTorque`))
  (bind _returnvalue (`KismetMathLibrary.Normal` (`KismetMathLibrary.MakeVector` (- (.x (`SceneComponent.K2_GetComponentLocation` (`self.Ball`))) (.x (`SceneComponent.K2_GetComponentLocation` (`self.Camera`)))) (- (.y (`SceneComponent.K2_GetComponentLocation` (`self.Ball`))) (.y (`SceneComponent.K2_GetComponentLocation` (`self.Camera`)))))))
  ;[1 1 1] Roll Control
  (set `self.directionTorque` (+ (* (`KismetMathLibrary.GreaterGreater_VectorRotator` _returnvalue (struct :`Yaw` 90.0)) (* AxisValue _rolltorque)) (* _returnvalue (* _rolltorque (stale `InputAxis|MoveRight` AxisValue) -1.0))) :!label _label)
  (if (<= 2500.0 (`KismetMathLibrary.VSize` (`SceneComponent.GetComponentVelocity` (`self.Ball`))))
    (`KismetMaterialLibrary.SetScalarParameterValue` "/Game/ASSET/IntensiveLine_material/MP_IntensiveLine.MP_IntensiveLine" "FlashFlag" 1.0)
    (else
      (`KismetMaterialLibrary.SetScalarParameterValue` "/Game/ASSET/IntensiveLine_material/MP_IntensiveLine.MP_IntensiveLine" "FlashFlag"))))

(event `InputAxis|MoveRight`
  (params (AxisValue :type "Float (single-precision)"))
  ;[1 1 1] Roll Control
  (goto _label))

(event `self.ReceiveTick`
  (params (DeltaSeconds :type "Float (single-precision)"))
  (bind _returnvalue (`SceneComponent.K2_GetComponentLocation` (`self.Ball`)))
  ;[1 1 1] Add Torque
  (if (< (`KismetMathLibrary.VSize` (`SceneComponent.GetComponentVelocity` (`self.Ball`))) (`self.maxMoveSpeed`))
    (bind _outhit (`KismetSystemLibrary.LineTraceSingle` :`Start` _returnvalue :`End` (+ _returnvalue (`KismetMathLibrary.MakeVector` 0.0 0.0 (* -1 (`self.ballRadius`)))) :`TraceChannel` "TraceTypeQuery1" :`TraceColor` (struct :`R` 0.12603 :`G` 1.0 :`B` 0.690565 :`A` 1.0) :`TraceHitColor` (struct :`R` 0.718223 :`G` 0.304925 :`B` 1.0 :`A` 1.0)))
    (if (`GameplayStatics.BreakHitResult` _outhit)
      (`PrimitiveComponent.AddTorqueInRadians` (`self.Ball`) (`self.directionTorque`) "None" false)
      ;[1 1 1] Update
      (bind _result (`/Engine/EditorBlueprintResources/StandardMacros.DecrementInt` (`self.speedUpTimeLimit`))
        (:`  `
          (if (not (< 0 _result))
            (`self.SpeedUpEnd`))
          (bind _result_2 (`/Engine/EditorBlueprintResources/StandardMacros.DecrementInt` (`self.SizeUpTimeLimit`))
            (:`  `
              (if (not (< 0 _result_2))
                (`self.SizeUpEnd`))
              (`/Engine/EditorBlueprintResources/StandardMacros.DecrementInt` (`self.invincibleTime`)))))))))

(event `InputAxis|Turn`
  (params (AxisValue :type "Float (single-precision)"))
  ;[1 1 1] CameraAngleControl
  (`self.AddControllerYawInput` AxisValue))

(event `InputAxis|LookUp`
  (params (AxisValue :type "Float (single-precision)"))
  ;[1 1 1] CameraAngleControl
  (`self.AddControllerPitchInput` AxisValue))

(fn `GetPlayerHP`
  (returns (PlayerHP :type Integer))
  (return (`self.PlayerHP`)))

(fn `GetSizeUpItem`
  (set `self.SizeUpTimeLimit` 900)
  (if (not (`self.SizeUpFlag`))
    (set `self.SizeUpFlag` true)
    (`SceneComponent.SetRelativeScale3D` (`self.Ball`) (* (`SceneComponent.K2_GetComponentScale` (`self.Ball`)) 2.0))
    (set `self.ballRadius` (* (`self.ballRadius`) 2.0))
    (set `self.RollTorque` (* (`self.RollTorque`) 1.5))
    (`AddComponent|NODE_AddAudioComponent-1`)))

(fn `GetSpeedUpItem`
  (set `self.speedUpTimeLimit` 900)
  (if (not (`self.SpeedUpFlag`))
    (set `self.SpeedUpFlag` true)
    (set `self.RollTorque` (* (`self.RollTorque`) 2.0))
    (set `self.maxMoveSpeed` (* (`self.maxMoveSpeed`) 2.0))
    (`AddComponent|NODE_AddAudioComponent-0`)))

(fn `PlayerDamage`
  (params (enemyMoveVector :type "Vector Structure (by ref)"))
  (if (`self.SizeUpFlag`)
    _
    (elif (<= (`self.invincibleTime`) 0)
      (set `self.invincibleTime` 60)
      (`PrimitiveComponent.AddImpulse` (`self.Ball`) (* (* (`KismetMathLibrary.MakeVector` (.x enemyMoveVector) (.y enemyMoveVector) 1.0) 2.0) 8000000) "None" false)
      (`/Engine/EditorBlueprintResources/StandardMacros.DecrementInt` (`self.PlayerHP`)))))

(fn `SetDefaultSize`
  (`SceneComponent.SetRelativeScale3D` (`self.Ball`) (3.0 3.0 3.0))
  (set `self.ballRadius` 200.0)
  (set `self.SizeUpFlag` false))

(fn `SetDefaultSpeed`
  (set `self.RollTorque` 1500000000.0)
  (set `self.maxMoveSpeed` 2000.0)
  (set `self.SpeedUpFlag` false))

(fn `SizeUpEnd`
  (bind _ball (`self.Ball`))
  (if (`self.SizeUpFlag`)
    (set `self.SizeUpFlag` false)
    (`SceneComponent.SetRelativeScale3D` _ball (/ (`SceneComponent.K2_GetComponentScale` _ball) 2.0))
    (set `self.ballRadius` (/ (`self.ballRadius`) 2.0))
    (set `self.RollTorque` (/ (`self.RollTorque`) 1.5))))

(fn `SpeedUpEnd`
  (if (`self.SpeedUpFlag`)
    (set `self.SpeedUpFlag` false)
    (set `self.RollTorque` (/ (`self.RollTorque`) 2.0))
    (set `self.maxMoveSpeed` (/ (`self.maxMoveSpeed`) 2.0))))

(fn `UserConstructionScript`)