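; ObjectSpawnerBP is a Stage 6 spawner actor that periodically and randomly spawns a scaled-down AI_Character_ at its own location.
; Tick accumulates time and, throughout each whole second divisible by SpawnTime, rolls every frame.
; A spawn needs the random roll to exactly match SpawnChance after both are scaled by SpawnMaxNun and truncated.
; A DoOnce caps spawns at one per window, resetting whenever the second is not divisible.
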(event `self.ReceiveTick`
  (params (DeltaSeconds :type "Float (single-precision)"))
  (set `self.Time` (+ DeltaSeconds (`self.Time`)))
  (if (== (mod (`KismetMathLibrary.FTrunc` (`self.Time`)) (`self.SpawnTime`)) 0)
    (if (== (`KismetMathLibrary.Conv_IntToDouble` (`KismetMathLibrary.FTrunc` (* (/ (`self.SpawnChance`) (`self.SpawnMaxNun`)) 100.0))) (`KismetMathLibrary.Conv_IntToDouble` (`KismetMathLibrary.FTrunc` (* (/ (+ (`KismetMathLibrary.Conv_IntToDouble` (`KismetMathLibrary.RandomInteger` 11)) (`KismetMathLibrary.RandomFloat`)) (`self.SpawnMaxNun`)) 100.0))))
      (`/Engine/EditorBlueprintResources/StandardMacros.DoOnce` false :!label _label
        (:`Completed`
          (`|SpawnActorFromClass` "/Game/AI/Actor/AI_Character_.AI_Character__C" (`KismetMathLibrary.MakeTransform` (`self.K2_GetActorLocation`) (struct) (0.75 0.75 0.75)) "Undefined" "OverrideRootScale" null null))))
    (else
      (goto _label :!via `Reset`))))

(fn `UserConstructionScript`)